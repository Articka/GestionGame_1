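; Day/night clock actor that shows the in-game time as text and swaps Sun and Moon component visibility by hour.
; Tick feeds SetTime, which advances one minute per real second or so, rolls hours over at midnight without changing the date, and refreshes the text.
; BeginPlay and each hour rollover update IsNight and visibility, handling only Autumn: night hours show Sun with IsNight false, daytime hours the reverse.
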(event EventBeginPlay
  (bind _sun (Variables|Default|GetSun))
  (bind _moon (Variables|Default|GetMoon))
  (Rendering|Components|TextRender|SetText (Variables|Default|GetHours) (Utilities|Text|ToText(String) (Utilities|String|Append (Utilities|String|ToString(Integer) (.hours (Variables|Default|GetHoursOfTheDay))) ":" (Utilities|String|ToString(Integer) (.minutes (Variables|Default|GetHoursOfTheDay))))))
  (switch string (.season (Variables|Default|GetHoursOfTheDay))
    (:Autumn
      (if (> (.hours (Variables|Default|GetHoursOfTheDay)) 19)
        (Variables|Default|SetHoursOfTheDay (Utilities|Struct|MakeHours_Season_Day_Struct (.hours (Variables|Default|GetHoursOfTheDay)) (.minutes (Variables|Default|GetHoursOfTheDay)) (.date (Variables|Default|GetHoursOfTheDay)) (.season (Variables|Default|GetHoursOfTheDay)) false) :!label _label)
        (Rendering|SetVisibility _sun true false)
        (Rendering|SetVisibility _moon false false)
        (elif (< (.hours (Variables|Default|GetHoursOfTheDay)) 7)
          (goto _label)
          (else
            (Variables|Default|SetHoursOfTheDay (Utilities|Struct|MakeHours_Season_Day_Struct (.hours (Variables|Default|GetHoursOfTheDay)) (.minutes (Variables|Default|GetHoursOfTheDay)) (.date (Variables|Default|GetHoursOfTheDay)) (.season (Variables|Default|GetHoursOfTheDay)) true))
            (Rendering|SetVisibility _moon true false)
            (Rendering|SetVisibility _sun false false)))))))

(event EventTick
  (params (DeltaSeconds :type Float%20%28single-precision%29))
  (CallFunction|SetTime DeltaSeconds))

(fn ConstructionScript)

(fn SetTime
  (params (DeltaTime :type Float%20%28single-precision%29))
  (bind _sun (Variables|Default|GetSun))
  (bind _moon (Variables|Default|GetMoon))
  (bind _output_get (Variables|Default|SetTimeOfTheDay (+ DeltaTime (Variables|Default|GetTimeOfTheDay))))
  (if (>= _output_get "1f")
    (Variables|Default|SetTimeOfTheDay 0.0)
    (bind _result (Math|Integer|IncrementInt (.minutes (Variables|Default|GetHoursOfTheDay)))
      (:%20%20
        (if (== _result 60)
          (if (== (+ (.hours (Variables|Default|GetHoursOfTheDay)) 1) 24)
            (Variables|Default|SetHoursOfTheDay (Utilities|Struct|MakeHours_Season_Day_Struct 0 0 (.date (Variables|Default|GetHoursOfTheDay)) (.season (Variables|Default|GetHoursOfTheDay)) (.isnight (Variables|Default|GetHoursOfTheDay))))
            (else
              (Variables|Default|SetHoursOfTheDay (Utilities|Struct|MakeHours_Season_Day_Struct (+ (.hours (Variables|Default|GetHoursOfTheDay)) 1) 0 (.date (Variables|Default|GetHoursOfTheDay)) (.season (Variables|Default|GetHoursOfTheDay)) (.isnight (Variables|Default|GetHoursOfTheDay))))))
          (switch string (.season (Variables|Default|GetHoursOfTheDay))
            (:Autumn
              (if (> (.hours (Variables|Default|GetHoursOfTheDay)) 19)
                (Variables|Default|SetHoursOfTheDay (Utilities|Struct|MakeHours_Season_Day_Struct (.hours (Variables|Default|GetHoursOfTheDay)) (.minutes (Variables|Default|GetHoursOfTheDay)) (.date (Variables|Default|GetHoursOfTheDay)) (.season (Variables|Default|GetHoursOfTheDay)) false) :!label _label)
                (Rendering|SetVisibility _sun true false)
                (Rendering|SetVisibility _moon false false)
                (elif (< (.hours (Variables|Default|GetHoursOfTheDay)) 7)
                  (goto _label)
                  (else
                    (Variables|Default|SetHoursOfTheDay (Utilities|Struct|MakeHours_Season_Day_Struct (.hours (Variables|Default|GetHoursOfTheDay)) (.minutes (Variables|Default|GetHoursOfTheDay)) (.date (Variables|Default|GetHoursOfTheDay)) (.season (Variables|Default|GetHoursOfTheDay)) true))
                    (Rendering|SetVisibility _moon true false)
                    (Rendering|SetVisibility _sun false false)))))))
        (if (not (<= (.minutes (Variables|Default|GetHoursOfTheDay)) 9))
          (Rendering|Components|TextRender|SetText (Variables|Default|GetHours) (Utilities|Text|ToText(String) (Utilities|String|Append (Utilities|String|ToString(Integer) (.hours (Variables|Default|GetHoursOfTheDay))) ":" (Utilities|String|ToString(Integer) _result))))
          (else
            (Rendering|Components|TextRender|SetText (Variables|Default|GetHours) (Utilities|Text|ToText(String) (Utilities|String|Append (Utilities|String|ToString(Integer) (.hours (Variables|Default|GetHoursOfTheDay))) ":" "0" (Utilities|String|ToString(Integer) _result))))))))))