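; Table actor showing localized FR/EN resource names and counts on text components, and setting IsTable on GameMaster while it overlaps its box.
; BeginPlay builds the text array and an ID-to-count map, seeded with placeholder 20 from only the "Doge" row.
; SetAllRessources, rerun by RefreshLanguage, uses each component's name as its data table row.
; The count lookup's found check is inverted; older hardcoded versions remain unreachable.
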(event OnComponentBeginOverlap(Box)
  (params (OverlappedComponent :type Primitive%20Component%20Object%20Reference) (OtherActor :type Actor%20Object%20Reference) (OtherComp :type Primitive%20Component%20Object%20Reference) (OtherBodyIndex :type Integer) (bFromSweep :type Boolean) (SweepResult :type Hit%20Result%20Structure%20%28by%20ref%29))
  ;[1 1 1] If player enter in box collision set is table
  (bind _asgame_master (Utilities|Casting|CastToGameMaster OtherActor))
  (Variables|/Game/Blueprint/GameMaster/GameMaster.GameMaster_C|SetIsTable _asgame_master true))

(event OnComponentEndOverlap(Box)
  (params (OverlappedComponent :type Primitive%20Component%20Object%20Reference) (OtherActor :type Actor%20Object%20Reference) (OtherComp :type Primitive%20Component%20Object%20Reference) (OtherBodyIndex :type Integer))
  ;[1 1 1] If player enter in box collision set is table
  (bind _asgame_master (Utilities|Casting|CastToGameMaster OtherActor))
  (Variables|/Game/Blueprint/GameMaster/GameMaster.GameMaster_C|SetIsTable _asgame_master false))

(event EventBeginPlay
  ;[1 1 1] Event begin play
  ;;[1 1 1] Get reference of actor village
  (bind _outactors (Actor|GetAllActorsOfClass "/Game/Blueprint/Village/Village.Village_C"))
  (Variables|Default|SetVillage (Utilities|Array|Get(acopy) _outactors))
  ;;[1 1 1] Set array of all text object
  (Variables|Default|SetAllTextObject (Utilities|Array|MakeArray (Variables|Default|GetWood) (Variables|Default|GetRock) (Variables|Default|GetScraps) (Variables|Default|GetScraps_Tech) (Variables|Default|GetWater) (Variables|Default|GetFood) (Variables|Default|GetMedicine) (Variables|Default|GetChicken) (Variables|Default|GetCow) (Variables|Default|GetIron) (Variables|Default|GetAnimals) (Variables|Default|GetRessources) (Variables|Default|GetConsommable)))
  (CallFunction|SetDictionaryOfRessources)
  (CallFunction|SetAllRessources))

(event EventRefreshLanguage
  ;[1 1 1] Event begin play
  (CallFunction|SetAllRessources))

(fn ConstructionScript)

(fn SetAllRessources
  ;[1 1 1] Set all text and number and change language
  (for _index (range 0 (Utilities|Array|Length (Variables|Default|GetAllTextObject)))
    (bind _returnvalue (Utilities|GetDataTableRow "/Game/Blueprint/DataTable/Language_And_SetID_-_Feuille_1__1_.Language_And_SetID_-_Feuille_1__1_" (Utilities|String|StringToName (Utilities|GetObjectName (Utilities|Array|Get(acopy) (Variables|Default|GetAllTextObject) _index))))
      (:then
        (bind _asgame_master_gamemode (Utilities|Casting|CastToGameMaster_Gamemode (Game|GetGameMode)))
        (bind _returnstringofnumber (CallFunction|GetNumberOfRessources (.ID (Utilities|Struct|BreakLanguage_And_SetID _returnvalue))))
        (switch Utilities|FlowControl|Switch|SwitchonLanguageOfGame (Variables|/Game/Blueprint/GameMaster/GameMaster_Gamemode.GameMaster_Gamemode_C|GetLanguage _asgame_master_gamemode)
          (:NewEnumerator0
            (Rendering|Components|TextRender|SetText (Utilities|Array|Get(acopy) (Variables|Default|GetAllTextObject) _index) (Utilities|Text|ToText(String) (Utilities|String|Append (.FR (Utilities|Struct|BreakLanguage_And_SetID _returnvalue)) _returnstringofnumber))))
          (:NewEnumerator1
            (Rendering|Components|TextRender|SetText (Utilities|Array|Get(acopy) (Variables|Default|GetAllTextObject) _index) (Utilities|Text|ToText(String) (Utilities|String|Append (.EN (Utilities|Struct|BreakLanguage_And_SetID _returnvalue)) _returnstringofnumber))))))))
  (return))

(fn GetNumberOfRessources
  (params (ID :type String))
  (bind _ressourcesandid (Variables|Default|GetRessourcesAndID))
  (bind (_value _returnvalue) (Utilities|Map|Find _ressourcesandid ID))
  (if (not _returnvalue)
    (return (Utilities|String|ToString(Integer) _value))
    (else
      (return ""))))

(fn SetDictionaryOfRessources
  (bind _returnvalue (Utilities|GetDataTableRow "/Game/Blueprint/DataTable/Language_And_SetID_-_Feuille_1__1_.Language_And_SetID_-_Feuille_1__1_" "Doge")
    (:then
      (for _index (range 0 (- (.NumberOfCollectibleObject (Utilities|Struct|BreakLanguage_And_SetID _returnvalue)) 1))
        (if (Utilities|Enum|NotEqual(Enum) (.ID (Utilities|Struct|BreakLanguage_And_SetID _returnvalue)) "")
          (Utilities|Map|Add (Variables|Default|GetRessourcesAndID) (.ID (Utilities|Struct|BreakLanguage_And_SetID _returnvalue)) 20)
          (Development|PrintString (Utilities|String|ToString(Integer) _index))))
      (Development|PrintString (Utilities|String|ToString(Integer) (Utilities|Map|Length (Variables|Default|GetRessourcesAndID))))
      (return))))